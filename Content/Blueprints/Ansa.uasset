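; Ansa is a trap actor that costs a life when it overlaps Hugo.
; On overlap it checks the other actor's name: a Hugo hit calls CallLifeLostED and pauses the world.
; Any other overlap runs the respawn-trigger check, waits a random few seconds, then moves the trap to GroundLevelPosition.
; Tick only calls the parent implementation, and the hit checks are defined outside this file.
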(event EventBeginPlay)

(event Collision|EventActorBeginOverlap
  (params (OtherActor :type Actor%20Object%20Reference))
  (bind _returnvalue (Utilities|GetObjectName OtherActor))
  ;[1 1 1] check if trap hits hugo
  (bind _hitresult (CallFunction|CheckHugoHit _returnvalue))
  (if _hitresult
    (Default|CallLifeLostED) ; GUI -message that life was lost
    (CallFunction|PauseWorld)
    (else
      (CallFunction|CheckRespawnHit _returnvalue) ; Check if trap hits respawn trigger
      (Utilities|FlowControl|Delay (Math|Random|RandomFloatinRange 1.0 4.0))
      (CallFunction|ResetTrapPosition))))

(event EventTick
  (params (DeltaSeconds :type Float%20%28single-precision%29))
  (|CallParentFunction 0.0))

(fn ConstructionScript)

(fn ResetTrapPosition
  (Transformation|SetActorLocation (Variables|Default|GetGroundLevelPosition) false false))