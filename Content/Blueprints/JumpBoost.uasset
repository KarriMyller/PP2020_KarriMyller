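; Jump boost pickup that temporarily raises the player character Hugo's jump velocity and tints his sprite blue.
; On Hugo's overlap it plays a sound, signals the collection, resets itself, then restores normal jump and color after a fixed delay.
; Any other overlap runs a respawn-trigger check, then resets position, scale and value after a random delay, regardless of the check's result.
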(event EventBeginPlay)

(event Collision|EventActorBeginOverlap
  (params (OtherActor :type Actor%20Object%20Reference))
  (bind _returnvalue (Utilities|GetObjectName OtherActor))
  ;[1 1 1] check if jump boost hit hugo
  (bind _hitresult (CallFunction|CheckHugoHit _returnvalue))
  (if _hitresult
    (CallFunction|ApplyEffect)
    ;[1 1 1] GUI -message that money was collected
    (Default|CallJumbBoostCollected)
    ;[1 1 1] reset jumpboost values
    (CallFunction|ResetPosition)
    (CallFunction|ResetScaleandValue)
    ;[1 1 1] Acguire Hugo blueprint
    (bind _ashugo (Utilities|Casting|CastToHugo (Game|GetPlayerCharacter 0)))
    (bind _output_get (Variables|Default|SetHugo _ashugo))
    ;[1 1 1] Set jump velocity when jump boost collected
    (Variables|/Script/Engine.CharacterMovementComponent|SetJumpZVelocity (Variables|/Script/Engine.Character|GetCharacterMovement _output_get) 8e+02)
    (Sprite|SetSpriteColor (Variables|/Script/Paper2D.PaperCharacter|GetSprite _output_get) "(R=0.013924,G=0.077523,B=0.515625,A=1.000000)")
    (Utilities|FlowControl|Delay 1e+01)
    (Variables|/Script/Engine.CharacterMovementComponent|SetJumpZVelocity (Variables|/Script/Engine.Character|GetCharacterMovement _output_get) 6e+02)
    (Sprite|SetSpriteColor (Variables|/Script/Paper2D.PaperCharacter|GetSprite _output_get) "(R=1.000000,G=1.000000,B=1.000000,A=1.000000)")
    (else
      ;[1 1 1] if not hugo -> check if hit respawntrigger
      (CallFunction|CheckRespawnHit _returnvalue)
      ;[1 1 1] reset jump boost values
      (Utilities|FlowControl|Delay (Math|Random|RandomFloatinRange 5.0 15.0))
      (CallFunction|ResetPosition)
      (CallFunction|ResetScaleandValue))))

(event EventTick
  (params (DeltaSeconds :type Float%20%28single-precision%29))
  (|CallParentFunction DeltaSeconds))

(fn ConstructionScript)

(fn ApplyEffect
  (Audio|PlaySound2D "/Game/Sounds/Jumboost_collected.Jumboost_collected" 1.0 1.0 0.0 0 0))