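; Moving collectible actor that can be reset with a random height and a random scale that sets its value.
; Tick offsets it by Speed times global time dilation, not delta time.
; PauseWorld flags Tick to briefly slow global time while raising the player's custom dilation, then restore both after a delay.
; Helper functions identify player and respawn-trigger hits by object name; no overlap logic calls them here.
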(event EventBeginPlay)

(event Collision|EventActorBeginOverlap
  (params (OtherActor :type Actor%20Object%20Reference)))

(event EventTick
  (params (DeltaSeconds :type Float%20%28single-precision%29))
  ;[1 1 1] Move the collectible
  (Transformation|AddActorWorldOffset (* (Variables|Default|GetSpeed) (Class|GameplayStatics|GetGlobalTimeDilation)))
  (if (!= (Variables|Default|GetDelayUntilNormalSpeed) 0)
    ;[1 1 1] set global time dilation and custom time dilation for playercharacter
    (Utilities|Time|SetGlobalTimeDilation 0.1)
    (Variables|/Script/Engine.Actor|SetCustomTimeDilation (Game|GetPlayerCharacter 0) 3.0)
    (Utilities|FlowControl|Delay 0.2)
    (Utilities|Time|SetGlobalTimeDilation 1.0)
    (Variables|/Script/Engine.Actor|SetCustomTimeDilation (Game|GetPlayerCharacter 0) 1.0)
    (Variables|Default|SetDelayUntilNormalSpeed 0)))

(fn ConstructionScript)

(fn ResetPosition
  (bind _initialposition (Variables|Default|GetInitialPosition))
  (bind (_x _y) (Math|Vector|BreakVector _initialposition))
  (Transformation|SetActorLocation (Math|Vector|MakeVector _x _y (Math|Random|RandomFloatinRange 2.5e+02 6e+02)) false false))

(fn ResetScaleandValue
  (bind _output_get (Variables|Default|Setscale (Math|Random|RandomFloatinRange 1.0 5.0)))
  (Transformation|SetActorScale3D (Math|Vector|MakeVector (/ _output_get 2.0) (/ _output_get 2.0) (/ _output_get 2.0)))
  (Variables|Default|Setvalue (Math|Float|Round (Variables|Default|Getscale))))

(fn CheckHugoHit
  (params (OtherObjectName :type String))
  (return (Utilities|Enum|Equal(Enum) OtherObjectName (Utilities|GetObjectName (Game|GetPlayerCharacter 0)))))

(fn CheckRespawnHit
  (params (OtherObjectName :type String))
  (return (Utilities|Enum|Equal(Enum) OtherObjectName (Variables|Default|GetRespawnTriggerName))))

(fn PauseWorld
  (Variables|Default|SetDelayUntilNormalSpeed 1))