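; Hugo is a flipbook-animated player character Blueprint that switches between running and jumping animations.
; Pressing Jump sets the jump flipbook and calls Jump on player character 0.
; A capsule hit against an actor tagged "surface" restores the run flipbook, serving as landing detection.
; BeginPlay sets the player controller to game-only input.
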(event OnComponentHit(CapsuleComponent)
  (params (HitComponent :type Primitive%20Component%20Object%20Reference) (OtherActor :type Actor%20Object%20Reference) (OtherComp :type Primitive%20Component%20Object%20Reference) (NormalImpulse :type Vector :default "0, 0, 0") (Hit :type Hit%20Result%20Structure%20%28by%20ref%29))
  (if (Actor|ActorHasTag OtherActor "surface")
    (Sprite|SetFlipbook (Variables|Default|GetSprite) "/Game/Flipbooks/RUN_3x4.RUN_3x4")))

(event EventBeginPlay
  (Input|SetInputModeGameOnly (Game|GetPlayerController 0)))

(event Collision|EventActorBeginOverlap
  (params (OtherActor :type Actor%20Object%20Reference)))

(event EventTick
  (params (DeltaSeconds :type Float%20%28single-precision%29)))

(event Input|ActionEvents|InputActionJump
  (params (Key :type Key%20Structure :default "None"))
  (:Pressed
    (Sprite|SetFlipbook (Variables|Default|GetSprite) "/Game/Flipbooks/jump.jump")
    (Character|Jump (Game|GetPlayerCharacter 0))))

(fn ConstructionScript)