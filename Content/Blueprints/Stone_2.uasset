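; Stone_2 is a stone obstacle that costs Hugo a life on overlap, firing the life-lost dispatcher and pausing the world.
; Other overlaps go through a respawn-trigger check.
; After either case, a random delay precedes a reset to a random X position at fixed Y and Z.
; Tick runs the parent's logic, then calls ChangeTime with a constant.
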(event EventBeginPlay)

(event Collision|EventActorBeginOverlap
  (params (OtherActor :type Actor%20Object%20Reference))
  (bind _returnvalue (Utilities|GetObjectName OtherActor))
  ;[1 1 1] check if stone hits hugo
  (bind _hitresult (CallFunction|CheckHugoHit _returnvalue))
  (if _hitresult
    (Default|CallLifeLostbyStoneED)
    (CallFunction|PauseWorld)
    (else
      ;[1 1 1] Reset position after random time delay
      (CallFunction|CheckRespawnHit _returnvalue) ; Check if trap hits respawn trigger
    ))
  (Utilities|FlowControl|Delay (Math|Random|RandomFloatinRange 6.0 12.0))
  (CallFunction|ResetStonePosition))

(event EventTick
  (params (DeltaSeconds :type Float%20%28single-precision%29))
  (|CallParentFunction 0.0)
  (CallFunction|ChangeTime 0.6))

(fn ConstructionScript)

(fn ResetStonePosition
  (bind _output_get (Variables|Default|SetInitialPosition "2000.000000,0.000000,180.000000"))
  (Transformation|SetActorLocation (Math|Vector|MakeVector (Math|Random|RandomFloatinRange 2e+03 4e+03) (.Y (Math|Vector|BreakVector _output_get)) (.Z (Math|Vector|BreakVector _output_get))) false false))